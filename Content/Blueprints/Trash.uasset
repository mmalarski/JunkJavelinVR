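; Trash is an actor that serves as a piece of litter, picking a random mesh from its Meshes array on BeginPlay.
; When it overlaps an actor whose class is exactly Javelin, it spawns a confetti Niagara effect at the mesh location and destroys itself.
; A sound call at the same location follows the destroy, with no sound asset shown.
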(event EventBeginPlay
  (Components|StaticMesh|SetStaticMesh (Variables|Default|GetStaticMesh) (.OutItem (Utilities|Array|Random (Variables|Default|GetMeshes)))))

(event Collision|EventActorBeginOverlap
  (params (OtherActor :type Actor%20Object%20Reference))
  (bind _staticmesh (Variables|Default|GetStaticMesh))
  (bind _returnvalue (Transformation|GetWorldLocation _staticmesh))
  (if (== (Utilities|GetClass OtherActor) "/Game/VRTemplate/Blueprints/Javelin.Javelin_C")
    (Niagara|SpawnSystematLocation "/Game/Particles/ConfettiEmitter_System.ConfettiEmitter_System" _returnvalue)
    (Actor|DestroyActor)
    (Audio|PlaySoundatLocation 0 _returnvalue "0, 0, 0" 1.0 1.0 0.0 0 0 0 0)))

(event EventTick
  (params (DeltaSeconds :type Float%20%28single-precision%29)))

(fn ConstructionScript)