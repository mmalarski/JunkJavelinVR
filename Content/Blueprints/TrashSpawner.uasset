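; TrashSpawner is an actor that refills an area with Trash actors whenever none remain overlapping it.
; Every Tick it checks its overlapping actors and, if no Trash is found, spawns a batch of fifty.
; Each piece gets a random X/Y point within the Box extent at the root's height and a random yaw, adjusting for collisions but always spawning.
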(event Custom|SpawnTrash
  (bind _box (Variables|Default|GetBox))
  (bind _defaultsceneroot (Variables|Default|GetDefaultSceneRoot))
  (bind _returnvalue (Transformation|GetWorldLocation _defaultsceneroot))
  (bind _boxextent (Variables|/Script/Engine.BoxComponent|GetBoxExtent _box))
  (bind _returnvalue_2 (Math|Random|RandomPointinBoundingBox (Math|Vector|MakeVector (.x _returnvalue) (.y _returnvalue) (.z _returnvalue)) _boxextent))
  (Game|SpawnActorfromClass "/Game/Blueprints/Trash.Trash_C" (Math|Transform|MakeTransform (Math|Vector|MakeVector (.x _returnvalue_2) (.y _returnvalue_2) (.z _returnvalue)) (Math|Rotator|MakeRotator 0.0 0.0 (Math|Conversions|ToFloat(Integer) (Math|Random|RandomInteger 360))) "1.000000,1.000000,1.000000") "AdjustIfPossibleButAlwaysSpawn" 0 0))

(event EventTick
  (params (DeltaSeconds :type Float%20%28single-precision%29))
  (if (<= (Utilities|Array|Length (Collision|GetOverlappingActors "/Game/Blueprints/Trash.Trash_C" :!class /Script/Engine.Actor)) 0)
    (for _index (range 0 49)
      (CallFunction|SpawnTrash))))

(fn ConstructionScript)